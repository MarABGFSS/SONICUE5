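; Shadow Rings memorabilia pickup whose collection releases a ChaserAI into the level.
; Tick spins the static mesh a fixed step each frame, not scaled by delta time.
; The PlayerAddMemo override runs the parent's logic, then spawns ChaserAI at a hardcoded world location, independent of where the pickup sits.
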(event EventBeginPlay
  (|CallParentFunction) ; This node is disabled and will not be called.\nDrag off pins to build functionality.
)

(event Collision|EventActorBeginOverlap
  (params (OtherActor :type Actor%20Object%20Reference))
  (|CallParentFunction OtherActor) ; This node is disabled and will not be called.\nDrag off pins to build functionality.
)

(event EventTick
  (params (DeltaSeconds :type Float%20%28single-precision%29))
  (|CallParentFunction DeltaSeconds)
  (Transformation|AddWorldRotation (Variables|Default|GetStaticMesh) "0.000000,1.000000,0.000000" false false))

(fn ConstructionScript
  (|CallParentFunction))

(fn PlayerAddMemo
  (|CallParentFunction)
  (Game|SpawnActorfromClass "/Game/2017X/ChaserAI.ChaserAI_C" (Math|Transform|MakeTransform "-15790.000000,-3780.000000,1200.000000" "0, 0, 0" "1.000000,1.000000,1.000000") "Undefined" "MultiplyWithRoot" 0 0))