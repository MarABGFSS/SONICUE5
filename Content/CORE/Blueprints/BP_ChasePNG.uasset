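; BP_ChasePNG is a chaser actor that starts audio on BeginPlay and rushes along the X axis toward a fixed end point, destroying any BP_FirstPersonCharacter it touches.
; A timeline lerps its location from the spawn point without sweeping.
; A second box, Box1, adjusts the timeline's play rate: the fast opening pace slows when the player enters it and partly speeds up when they leave, giving simple rubber-banding.
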(event OnComponentBeginOverlap(Box)
  (params (OverlappedComponent :type Primitive%20Component%20Object%20Reference) (OtherActor :type Actor%20Object%20Reference) (OtherComp :type Primitive%20Component%20Object%20Reference) (OtherBodyIndex :type Integer) (bFromSweep :type Boolean) (SweepResult :type Hit%20Result%20Structure%20%28by%20ref%29))
  (bind _asbp_first_person_character (Utilities|Casting|CastToBP_FirstPersonCharacter OtherActor))
  (Actor|DestroyActor _asbp_first_person_character))

(event OnComponentEndOverlap(Box1)
  (params (OverlappedComponent :type Primitive%20Component%20Object%20Reference) (OtherActor :type Actor%20Object%20Reference) (OtherComp :type Primitive%20Component%20Object%20Reference) (OtherBodyIndex :type Integer))
  (Utilities|Casting|CastToBP_FirstPersonCharacter OtherActor)
  (Components|Timeline|SetPlayRate (Variables|Default|GetChas) 1.5))

(event OnComponentBeginOverlap(Box1)
  (params (OverlappedComponent :type Primitive%20Component%20Object%20Reference) (OtherActor :type Actor%20Object%20Reference) (OtherComp :type Primitive%20Component%20Object%20Reference) (OtherBodyIndex :type Integer) (bFromSweep :type Boolean) (SweepResult :type Hit%20Result%20Structure%20%28by%20ref%29))
  (Utilities|Casting|CastToBP_FirstPersonCharacter OtherActor)
  (Components|Timeline|SetPlayRate (Variables|Default|GetChas) 1.0))

(event EventBeginPlay
  (Components|Timeline|SetPlayRate (Variables|Default|GetChas) 2.3)
  (Audio|Components|Audio|Play (Variables|Default|GetAudio) 0.0)
  (Variables|Default|SetinitLoc (Transformation|GetActorLocation))
  (Variables|Default|SetCube (Variables|Default|GetCube))
  (bind _alpha (Timeline|Chas PlayFromStart)
    (:Update
      (Transformation|SetActorLocation (Math|Vector|Lerp(Vector) (Variables|Default|GetinitLoc) (Math|Vector|MakeVector 2.817e+04 (.Y (Math|Vector|BreakVector (Variables|Default|GetinitLoc))) (.Z (Math|Vector|BreakVector (Variables|Default|GetinitLoc)))) _alpha) false false))))

(fn ConstructionScript)