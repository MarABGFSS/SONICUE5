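; BP_BasementDoor is a sliding double door that stays locked until the emerald is collected.
; CollectEmerald sets a flag, and a first-person character overlapping the trigger box then opens the door.
; Two timelines slide the left and right panels along local Y, and leaving the box reverses both to close it.
; The close on exit does not check the emerald flag.
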(event OnComponentBeginOverlap(Box)
  (params (OverlappedComponent :type Primitive%20Component%20Object%20Reference) (OtherActor :type Actor%20Object%20Reference) (OtherComp :type Primitive%20Component%20Object%20Reference) (OtherBodyIndex :type Integer) (bFromSweep :type Boolean) (SweepResult :type Hit%20Result%20Structure%20%28by%20ref%29))
  ;[1 1 1] door
  (if (Variables|Default|GetEmeraldCollected)
    (Utilities|Casting|CastToBP_FirstPersonCharacter OtherActor)
    (CallFunction|OpenDoor)))

(event OnComponentEndOverlap(Box)
  (params (OverlappedComponent :type Primitive%20Component%20Object%20Reference) (OtherActor :type Actor%20Object%20Reference) (OtherComp :type Primitive%20Component%20Object%20Reference) (OtherBodyIndex :type Integer))
  ;[1 1 1] door
  (Utilities|Casting|CastToBP_FirstPersonCharacter OtherActor)
  (CallFunction|CloseDoor))

(event Custom|CollectEmerald
  (Variables|Default|SetEmeraldCollected true))

(event Custom|OpenDoor
  ;[1 1 1] door
  (Utilities|FlowControl|Sequence
    (:then_0
      (bind _doorleftmovebitch (Timeline|Timeline PlayFromStart)
        (:Update
          (Transformation|SetRelativeLocation (Variables|Default|GetLeftDoor) (Math|Vector|MakeVector 0.0 (.x _doorleftmovebitch) 0.0) false false))))
    (:then_1
      (bind _newtrack_0 (Timeline|Timeline_0 PlayFromStart)
        (:Update
          (Transformation|SetRelativeLocation (Variables|Default|Getrightdoor) (Math|Vector|MakeVector 0.0 _newtrack_0 0.0) false false))))))

(event Custom|CloseDoor
  ;[1 1 1] door
  (Utilities|FlowControl|Sequence
    (:then_0
      (bind _doorleftmovebitch (Timeline|Timeline Reverse)
        (:Update
          (Transformation|SetRelativeLocation (Variables|Default|GetLeftDoor) (Math|Vector|MakeVector 0.0 (.x _doorleftmovebitch) 0.0) false false))))
    (:then_1
      (bind _newtrack_0 (Timeline|Timeline_0 Reverse)
        (:Update
          (Transformation|SetRelativeLocation (Variables|Default|Getrightdoor) (Math|Vector|MakeVector 0.0 _newtrack_0 0.0) false false))))))

(fn ConstructionScript)