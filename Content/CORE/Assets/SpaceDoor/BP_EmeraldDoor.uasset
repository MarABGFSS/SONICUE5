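; Keycard-locked sliding double door that opens when the first-person character enters its trigger box.
; CollectKeycard sets the unlock flag, which box overlap checks before calling OpenDoor; leaving the box calls CloseDoor without that check.
; Two timelines slide the panels along relative Y, cross-named so DoorLeft drives RightDoor.
; Opening always plays from the start, while closing reverses both timelines.
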(event OnComponentBeginOverlap(Box)
  (params (OverlappedComponent :type Primitive%20Component%20Object%20Reference) (OtherActor :type Actor%20Object%20Reference) (OtherComp :type Primitive%20Component%20Object%20Reference) (OtherBodyIndex :type Integer) (bFromSweep :type Boolean) (SweepResult :type Hit%20Result%20Structure%20%28by%20ref%29))
  ;[1 1 1] door
  (if (Variables|Default|GetKeycardCollected)
    (Utilities|Casting|CastToBP_FirstPersonCharacter OtherActor)
    (CallFunction|OpenDoor)))

(event OnComponentEndOverlap(Box)
  (params (OverlappedComponent :type Primitive%20Component%20Object%20Reference) (OtherActor :type Actor%20Object%20Reference) (OtherComp :type Primitive%20Component%20Object%20Reference) (OtherBodyIndex :type Integer))
  ;[1 1 1] door
  (Utilities|Casting|CastToBP_FirstPersonCharacter OtherActor)
  (CallFunction|CloseDoor))

(event Custom|CollectKeycard
  (Variables|Default|SetKeycardCollected true))

(event Custom|OpenDoor
  ;[1 1 1] door
  (Utilities|FlowControl|Sequence
    (:then_0
      (bind _doorleftmovebitch (Timeline|DoorLeft PlayFromStart)
        (:Update
          (Transformation|SetRelativeLocation (Variables|Default|GetRightDoor) (Math|Vector|MakeVector 0.0 (.x _doorleftmovebitch) 0.0) false false))))
    (:then_1
      (bind _doorrightmovebitch (Timeline|Timeline PlayFromStart)
        (:Update
          (Transformation|SetRelativeLocation (Variables|Default|GetLeftDoor) (Math|Vector|MakeVector 0.0 (.x _doorrightmovebitch) 0.0) false false))))))

(event Custom|CloseDoor
  ;[1 1 1] door
  (Utilities|FlowControl|Sequence
    (:then_0
      (bind _doorleftmovebitch (Timeline|DoorLeft Reverse)
        (:Update
          (Transformation|SetRelativeLocation (Variables|Default|GetRightDoor) (Math|Vector|MakeVector 0.0 (.x _doorleftmovebitch) 0.0) false false))))
    (:then_1
      (bind _doorrightmovebitch (Timeline|Timeline Reverse)
        (:Update
          (Transformation|SetRelativeLocation (Variables|Default|GetLeftDoor) (Math|Vector|MakeVector 0.0 (.x _doorrightmovebitch) 0.0) false false))))))

(event EventBeginPlay)

(event Collision|EventActorBeginOverlap
  (params (OtherActor :type Actor%20Object%20Reference)))

(fn ConstructionScript)