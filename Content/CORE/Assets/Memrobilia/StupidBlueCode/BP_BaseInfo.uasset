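; Base actor for interactable info points that present a text sequence as an information or dialogue display.
; A world-space prompt widget turns toward the player while WidgetAlive is set, appearing and hiding through the interaction events.
; StartInteract creates the screen widget mapped to the selected interaction type, then steps through TextSequence on repeat interactions.
; StopInteract, or the index running out, removes the display and resets the index.
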(event EventBeginPlay
  (bind _aswb_prompt (Utilities|Casting|CastToWB_Prompt (UserInterface|GetWidget (Variables|Default|GetWB_Prompt))))
  (Variables|Default|SetWidget _aswb_prompt))

(event Collision|EventActorBeginOverlap
  (params (OtherActor :type Actor%20Object%20Reference)))

(event EventCanInteract
  (Default|ShowUp (Variables|Default|GetWidget)))

(event EventStopInteract
  (Default|FuckOff (Variables|Default|GetWidget))
  (Variables|Default|GetDisplayedWidget
    (:then
      (CallFunction|ResetUI))
    (:else)))

(event EventStartInteract
  (Default|FuckOff (Variables|Default|GetWidget))
  (Variables|Default|GetDisplayedWidget
    (:then
      (CallFunction|UpdateTexttoDisplay)
      (CallFunction|SetTexttoDisplay))
    (:else
      (CallFunction|AddWidgettoViewport)
      (CallFunction|SetTexttoDisplay))))

(event EventTick
  (params (DeltaSeconds :type Float%20%28single-precision%29))
  (if (Variables|Default|GetWidgetAlive)
    (Transformation|SetRelativeRotation (Variables|Default|GetWB_Prompt) (Math|Rotator|FindLookatRotation (Transformation|GetWorldLocation (Variables|Default|GetWB_Prompt)) (Transformation|GetActorLocation (Game|Player|GetPlayerPawn 0))) false false)))

(fn ConstructionScript)

(fn UpdateTexttoDisplay
  (if (< (Variables|Default|GetTextToDisplay) (- (Utilities|Array|Length (Variables|Default|GetTextSequence)) 0))
    (Math|Integer|IncrementInt (Variables|Default|GetTextToDisplay))
    (else
      (CallFunction|ResetUI))))

(fn ResetUI
  (Widget|RemovefromParent (Variables|Default|GetDisplayedWidget))
  (Variables|Default|SetDisplayedWidget 0)
  (Rendering|SetVisibility (Variables|Default|GetWB_Prompt) true false)
  (Variables|Default|SetTextToDisplay 0))

(fn SetTexttoDisplay
  (bind _aswb_information_display (Utilities|Casting|CastToWB_InformationDisplay (Variables|Default|GetDisplayedWidget))
    (:then
      (Variables|/Game/CORE/Assets/Memrobilia/StupidBlueCode/WB_InformationDisplay.WB_InformationDisplay_C|SetTextToDisplay _aswb_information_display (Utilities|Array|Get(acopy) (Variables|Default|GetTextSequence) (Variables|Default|GetTextToDisplay))))
    (:CastFailed
      (bind _aswb_dialogue_display (Utilities|Casting|CastToWB_DialogueDisplay (Variables|Default|GetDisplayedWidget)))
      (Variables|/Game/CORE/Assets/Memrobilia/StupidBlueCode/WB_DialogueDisplay.WB_DialogueDisplay_C|SetTextToDisplay _aswb_dialogue_display (Utilities|Array|Get(acopy) (Variables|Default|GetTextSequence) (Variables|Default|GetTextToDisplay))))))

(fn AddWidgettoViewport
  (bind _interactiontypemap (Variables|Default|GetInteractionTypeMap))
  (bind _selectedinteractiontype (Variables|Default|GetSelectedInteractionType))
  (bind (_value _returnvalue) (Utilities|Map|Find _interactiontypemap _selectedinteractiontype))
  (if _returnvalue
    (bind _output_get (Variables|Default|SetWidgetToDisplay _value))
    (bind _returnvalue_2 (UserInterface|CreateWidget _output_get))
    (Utilities|IsValid _returnvalue_2
      (:Is%20Valid
        (bind _output_get_2 (Variables|Default|SetDisplayedWidget _returnvalue_2))
        (UserInterface|Viewport|AddtoViewport _output_get_2 0)))))